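; Game mode that sets global time dilation from the average of every player's requested value.
; It tracks Tale4PlayerStates on login and logout, then each Tick averages their clamped TDValue into GlobalTimeDilationReplicated when it changes.
; That variable's RepNotify applies the clamped value as global time dilation and audio pitch modulation, and prints it on screen.
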(event EventBeginPlay
  (|CallParentFunction) ; This node is disabled and will not be called.\nDrag off pins to build functionality.
)

(event EventPostLogin
  (params (NewPlayer :type Player%20Controller%20Object%20Reference))
  (bind _astale_4player_state (Utilities|Casting|CastToTale4PlayerState (Variables|/Script/Engine.Controller|GetPlayerState NewPlayer)))
  (Utilities|Array|Add (Variables|Default|GetPlayerStates) _astale_4player_state))

(event EventOnLogout
  (params (ExitingController :type Controller%20Object%20Reference))
  (bind _playerstates (Variables|Default|GetPlayerStates))
  (bind _astale_4player_state (Utilities|Casting|CastToTale4PlayerState (Variables|/Script/Engine.Controller|GetPlayerState ExitingController)))
  (if (Utilities|Array|ContainsItem _playerstates _astale_4player_state)
    (Utilities|Array|RemoveIndex _playerstates (Utilities|Array|FindItem _playerstates _astale_4player_state))))

(event EventTick
  (params (DeltaSeconds :type Float%20%28single-precision%29))
  (|CallParentFunction DeltaSeconds)
  (bind _returnvalue (CallFunction|TimeDilationTick))
  (if (!= (Variables|Default|GetGlobalTimeDilationReplicated) _returnvalue)
    (Variables|Default|SetGlobalTimeDilationReplicated _returnvalue)))

(fn ConstructionScript
  (|CallParentFunction))

(fn TimeDilationTick
  (if (Utilities|Array|IsValidIndex (Variables|Default|GetPlayerStates))
    (for _array_element (Variables|Default|GetPlayerStates)
      (LocalVariables|SetTD_Local (+ (Math|Float|Clamp(Float) (Variables|/Game/Code/Tale4PlayerState.Tale4PlayerState_C|GetTD_Value _array_element)) (LocalVariables|GetTD_Local))))
    (return (/ (LocalVariables|GetTD_Local) (Utilities|Array|Length (Variables|Default|GetPlayerStates))))))

(fn OnRepGlobalTimeDilationReplicated
  (bind _globaltimedilationreplicated (Variables|Default|GetGlobalTimeDilationReplicated))
  (bind _returnvalue (Math|Float|Clamp(Float) _globaltimedilationreplicated 0.01))
  (Utilities|Time|SetGlobalTimeDilation _returnvalue)
  (Development|PrintString (Utilities|String|ToString(Float) _returnvalue) true true "(R=1.000000,G=0.048107,B=0.000000,A=1.000000)" 0.0)
  (Class|GameplayStatics|SetGlobalPitchModulation _returnvalue 0.1))