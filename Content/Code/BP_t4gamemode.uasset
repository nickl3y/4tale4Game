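; Game mode that runs a fixed-length timed match on the server.
; On BeginPlay the authority starts a one-shot timer that pauses the game when it expires.
; When a player logs in, it passes the timer's remaining time to that player's Tale4PlayerState so the player state knows how long is left.
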(event Custom|StopGame
  (Game|SetGamePaused true))

(event EventBeginPlay
  (Networking|SwitchHasAuthority
    (:Authority
      (bind _returnvalue (Utilities|Time|SetTimerbyEvent (delegate Custom|StopGame) 25.0))
      (Variables|Default|SetGameTimer _returnvalue))))

(event EventPostLogin
  (params (NewPlayer :type Player%20Controller%20Object%20Reference))
  (bind _astale_4player_state (Utilities|Casting|CastToTale4PlayerState (Variables|/Script/Engine.Controller|GetPlayerState NewPlayer)))
  (Default|ReceiveRemaining _astale_4player_state (Utilities|Time|GetTimerRemainingTimebyHandle (Variables|Default|GetGameTimer))))

(fn ConstructionScript)