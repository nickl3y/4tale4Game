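; BP_TimelineActor is a throwaway helper actor that runs a timeline of configurable duration and reports its progress through Update and Finished calls.
; On BeginPlay it applies the IgnoreTimeDilation setting, sets the play rate to the inverse of Time and plays from the start.
; Each tick of the timeline passes its float value to Update.
; On completion it calls Finished and destroys itself.
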(event EventBeginPlay
  (Class|TimelineComponent|SetIgnoreTimeDilation (Variables|Default|GetTimeline) (Variables|Default|GetIgnoreTimeDilation))
  (Components|Timeline|SetPlayRate (Variables|Default|GetTimeline) (/ 1.0 (Variables|Default|GetTime)))
  (bind _float (Timeline|Timeline PlayFromStart)
    (:Update
      (Default|CallUpdate _float))
    (:Finished
      (Default|CallFinished)
      (Actor|DestroyActor))))

(fn ConstructionScript)